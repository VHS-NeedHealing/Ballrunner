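; Cannon01 is an automatic cannon actor that fires projectiles repeatedly from the moment play begins.
; Each cycle waits a set Duration, then spawns the configured Projectile class at the Arrow component's position and rotation with an adjustable scale.
; A timeline then animates the Cannonarm along its local Y axis, and its finish restarts the cycle, so the firing interval is the delay plus the animation length.
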(event `self.ReceiveBeginPlay`
  (bind _arrow (`self.Arrow`))
  (`KismetSystemLibrary.Delay` (`self.Duration`) :!label _label)
  (`|SpawnActorFromClass` "/Game/Blueprints/cannon/projectile.projectile_C" (`KismetMathLibrary.MakeTransform` (`SceneComponent.K2_GetComponentLocation` _arrow) (`SceneComponent.K2_GetComponentRotation` _arrow) (`KismetMathLibrary.Conv_DoubleToVector` (`self.cannon projectile scale`))) "Undefined" "OverrideRootScale" null null)
  (bind (_direction _newtrack_0) (`Timeline|Timeline_0` :!via `PlayFromStart`)
    (:`Update`
      (`SceneComponent.K2_SetRelativeLocation` (`self.cannonarm`) (`KismetMathLibrary.MakeVector` 0.0 _newtrack_0) false false))
    (:`Finished`
      (goto _label))))

(fn `UserConstructionScript`)