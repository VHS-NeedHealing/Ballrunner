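; Collectible crystal that the player pawn picks up by overlapping its sphere.
; The overlap plays a timeline whose two curves pull the actor toward the player's live position and shrink it to zero, lerping from current values on each update.
; When the timeline finishes, the actor is destroyed and a 2D pickup sound plays.
; Overlaps from any other actor only print a debug message.
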(event `self.Sphere.OnComponentBeginOverlap`
  (params (OverlappedComponent :type "PrimitiveComponent Object Reference") (OtherActor :type "Actor Object Reference") (OtherComp :type "PrimitiveComponent Object Reference") (OtherBodyIndex :type Integer) (bFromSweep :type Boolean) (SweepResult :type "HitResult Structure (by ref)"))
  ;[1 1 1] Znajdzki zbieranie
  (if (== OtherActor (`GameplayStatics.GetPlayerPawn` 0))
    (bind (_direction _collectiblemovement _collectiblescale) (`Timeline|Timeline_0`)
      (:`Update`
        (`self.K2_SetActorLocation` (`KismetMathLibrary.VLerp` (`self.K2_GetActorLocation`) (`self.K2_GetActorLocation` (`GameplayStatics.GetPlayerPawn` 0)) _collectiblemovement))
        (`self.SetActorScale3D` (`KismetMathLibrary.VLerp` (`self.GetActorScale3D`) (0.0 0.0 0.0) _collectiblescale)))
      (:`Finished`
        (`self.K2_DestroyActor`)
        (`GameplayStatics.SpawnSound2D` "/Game/soundeffects/60900f7a-dfb5-4af1-92e2-2e8745145f8d.60900f7a-dfb5-4af1-92e2-2e8745145f8d" 1.0 1.0 0.0 null)))
    (else
      (`KismetSystemLibrary.PrintString` "Przeciwnik chcial zabrac krysztal"))))

(fn `UserConstructionScript`)